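; BP_Action_CastSpell is a player action in the CombatSetup set that casts a spell from the selected tile onto a target tile.
; ExecuteAction delegates the cast to the CombatSystem, which is responsible for validating it.
; It then resets the selected unit's AP, MP, RP, per-turn cast counts and spell cooldowns if that unit is valid, regardless of the cast's result.
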(event EventBeginPlay
  (|CallParentFunction) ; This node is disabled and will not be called.\nDrag off pins to build functionality.
)

(event Collision|EventActorBeginOverlap
  (params (OtherActor :type Actor%20Object%20Reference))
  (|CallParentFunction OtherActor) ; This node is disabled and will not be called.\nDrag off pins to build functionality.
)

(event EventTick
  (params (DeltaSeconds :type Float%20%28single-precision%29))
  (|CallParentFunction DeltaSeconds) ; This node is disabled and will not be called.\nDrag off pins to build functionality.
)

(fn ConstructionScript
  (|CallParentFunction))

(fn ExecuteAction
  (params (Index :type Int%20Point%20Structure))
  (bind _playeractions (Variables|Default|GetPlayerActions))
  (bind _selectedunit (Variables|/Game/TurnBasedTactic/Blueprints/Core/Player/BP_PlayerActions.BP_PlayerActions_C|GetSelectedUnit _playeractions))
  ;[0 0 0] [EN] Ask the CombatSystem to cast the spell. That way, it can validate that the spell can be casted before doing it
  ; [FR] Demande au CombatSystem de lancer le sort. De cette façon, il peut valider que le sort peut vraiment être lancé avant de le faire
  (Default|CastSpell (Variables|/Game/TurnBasedTactic/Blueprints/Core/Player/BP_PlayerActions.BP_PlayerActions_C|GetCombatSystem (Variables|Default|GetPlayerActions)) (Variables|Default|GetSpell) (Variables|/Game/TurnBasedTactic/Blueprints/Core/Player/BP_PlayerActions.BP_PlayerActions_C|GetSelectedTile (Variables|Default|GetPlayerActions)) Index)
  (Utilities|IsValid _selectedunit
    (:Is%20Valid
      (Default|ResetAp _selectedunit)
      (Default|ResetMp _selectedunit)
      (Default|ResetRp _selectedunit)
      (Default|ResetSpellsCastCountThisTurn _selectedunit)
      (Default|ResetSpellsCooldown _selectedunit))))