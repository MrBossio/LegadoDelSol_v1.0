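; Spell animation actor for the Uscovilca spell in a turn-based tactics game, showing a dark red and black wave at the target tile.
; It teleports to that tile and plays a sound while a timeline scales the effect and drives the opacity of three meshes.
; Early in the timeline, a DoOnce reports a hit on every attacked tile, and the timeline's end completes the animation.
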(event EventEventPlaySpellAnimation
  (bind _targetindex (Variables|Default|GetTargetIndex))
  (bind _transform (CallFunction|GetTileTransform _targetindex))
  (Transformation|SetActorLocation (.location _transform) false false)
  (Utilities|FlowControl|Sequence
    (:then_0
      (bind (_direction _opacity _scale) (Timeline|Timeline_DarkWave PlayFromStart)
        (:Update
          (Transformation|SetRelativeScale3D (Variables|Default|GetAnim_Scale) _scale)
          (Rendering|Material|SetScalarParameterValueonMaterials (Variables|Default|GetStaticMesh1) "Opacity" _opacity)
          (if (>= (Components|Timeline|GetPlaybackPosition (Variables|Default|GetTimeline_DarkWave)) 0.2)
            (Utilities|FlowControl|DoOnce false
              (:Completed
                (for _array_element (Variables|Default|GetAttackedIndexes)
                  (Default|CallOnSpellAnimationHitTile self _array_element))))))
        (:Finished
          (CallFunction|EventCompleteSpellAnimation))))
    (:then_1
      (Audio|PlaySoundatLocation "/Game/HumanVocalizations/Custom/sfx-spell-ray-fire.sfx-spell-ray-fire" (.location _transform) "0, 0, 0" 1.0 1.0 0.0 0 0 0 0))))

(fn ConstructionScript
  (|CallParentFunction)
  (Rendering|Material|SetVectorParameterValueonMaterials (Variables|Default|GetStaticMesh) "Color" (Math|Conversions|ToVector(LinearColor) "(R=0.364583,G=0.000000,B=0.000000,A=1.000000)"))
  (Rendering|Material|SetVectorParameterValueonMaterials (Variables|Default|GetStaticMesh1) "Color" (Math|Conversions|ToVector(LinearColor) "(R=0.000000,G=0.000000,B=0.000000,A=1.000000)"))
  (Rendering|Material|SetVectorParameterValueonMaterials (Variables|Default|GetStaticMesh2) "Color" (Math|Conversions|ToVector(LinearColor) "(R=0.000000,G=0.000000,B=0.000000,A=1.000000)")))