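; Spell animation Blueprint that plays a buff effect on a target tile in the turn-based tactics game.
; It moves to the tile, sets an icon on its widget component and plays a magic sound.
; A timeline animates the widget's height, draw size and opacity, signals the tile hit once shortly after starting, and completes the spell animation when finished.
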(event EventEventPlaySpellAnimation
  (bind _widget_0 (Variables|Default|GetWidget_0))
  (bind _targetindex (Variables|Default|GetTargetIndex))
  (bind _transform (CallFunction|GetTileTransform _targetindex))
  (Transformation|SetActorLocation (.location _transform) false false)
  (bind _output_get (Variables|Default|SetW_Image (.AsWBP%20Image (Utilities|Casting|CastToWBP_Image (UserInterface|GetUserWidgetObject (Variables|Default|GetWidget_0))))))
  (Appearance|SetBrushfromTexture (Variables|/Game/TurnBasedTactic/Blueprints/Core/Combat/Spells/SpellAnimations/Components/WBP_Image.WBP_Image_C|GetImage_Component _output_get) "/Game/TurnBasedTactic/Blueprints/Core/Combat/Spells/SpellAnimations/Assets/TX_Icon_Spells_X.TX_Icon_Spells_X" false)
  (Utilities|FlowControl|Sequence
    (:then_0
      (bind (_direction _locationz _drawsize _opacity) (Timeline|Timeline_RunChickenRun PlayFromStart)
        (:Update
          (Transformation|SetRelativeLocation _widget_0 (Math|Vector|MakeVector 0.0 0.0 _locationz) false false)
          (Class|WidgetComponent|SetDrawSize _widget_0 (Math|Vector2D|MakeVector2D _drawsize _drawsize))
          (Widget|SetRenderOpacity (Variables|Default|GetW_Image) _opacity)
          (if (>= (Components|Timeline|GetPlaybackPosition (Variables|Default|GetTimeline_RunChickenRun)) 0.2)
            (Utilities|FlowControl|DoOnce false
              (:Completed
                (Default|CallOnSpellAnimationHitTile self (Variables|Default|GetTargetIndex))))))
        (:Finished
          (CallFunction|EventCompleteSpellAnimation))))
    (:then_1
      (Audio|PlaySoundatLocation "/Game/HumanVocalizations/Custom/sfx-magic5.sfx-magic5" (.location _transform) "0, 0, 0" 1.0 1.0 0.0 0 0 0 0))))

(fn ConstructionScript
  (|CallParentFunction))