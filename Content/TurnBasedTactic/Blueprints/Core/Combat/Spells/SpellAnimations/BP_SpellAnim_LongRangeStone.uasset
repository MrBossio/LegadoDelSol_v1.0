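; Spell animation Blueprint for a long-range stone attack in the turn-based tactics game, moving the projectile from an origin tile to a target tile.
; It faces the target and plays an attack voice while a timeline lerps its position with a height offset, driving pitch and scale.
; The timeline, named for a long-range arrow, signals the tile hit once near 0.6 seconds and completes the animation when finished.
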(event EventEventPlaySpellAnimation
  (bind _anim_rotationscale (Variables|Default|GetAnim_RotationScale))
  (bind _originindex (Variables|Default|GetOriginIndex))
  (bind _transform (CallFunction|GetTileTransform _originindex))
  (Transformation|SetActorLocationAndRotation (.location _transform) (Math|Rotator|FindLookatRotation (Math|Conversions|ToVector(Vector2D) (Math|Conversions|ToVector2D(IntPoint) (Variables|Default|GetOriginIndex))) (Math|Conversions|ToVector(Vector2D) (Math|Conversions|ToVector2D(IntPoint) (Variables|Default|GetTargetIndex)))))
  (Utilities|FlowControl|Sequence
    (:then_0
      (bind (_direction _locationalpha _locationz _rotationy _scale) (Timeline|Timeline_LongRangeArrow PlayFromStart)
        (:Update
          (Transformation|SetActorLocation (+ (Math|Vector|Lerp(Vector) (.location (CallFunction|GetTileTransform (Variables|Default|GetOriginIndex))) (.location (CallFunction|GetTileTransform (Variables|Default|GetTargetIndex))) _locationalpha) (Math|Vector|MakeVector 0.0 0.0 _locationz)) false false)
          (Transformation|SetRelativeRotation _anim_rotationscale (Math|Rotator|MakeRotator 0.0 _rotationy 0.0) false false)
          (Transformation|SetRelativeScale3D _anim_rotationscale (Math|Conversions|ToVector(Float) _scale))
          (if (>= (Components|Timeline|GetPlaybackPosition (Variables|Default|GetTimeline_LongRangeArrow)) 0.6)
            (Utilities|FlowControl|DoOnce false
              (:Completed
                (Default|CallOnSpellAnimationHitTile self (Variables|Default|GetTargetIndex))))))
        (:Finished
          (CallFunction|EventCompleteSpellAnimation))))
    (:then_1
      (Audio|PlaySoundatLocation "/Game/HumanVocalizations/HumanMaleB/Wavs/voice_male_b_attack_set1_01.voice_male_b_attack_set1_01" (.location _transform) "0, 0, 0" 1.0 1.0 0.0 0 0 0 0))))

(fn ConstructionScript
  (|CallParentFunction))