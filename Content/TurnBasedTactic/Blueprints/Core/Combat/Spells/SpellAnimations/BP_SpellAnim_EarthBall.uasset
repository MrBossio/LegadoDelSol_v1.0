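; Spell animation Blueprint for the EarthBall spell in a turn-based tactics game, showing three tinted stones flying from the origin tile to the target tile.
; A timeline drives the position, height offset, stone opacity and scale while a cast sound plays at the origin.
; Partway through, a DoOnce reports a hit on every attacked tile, and the timeline's end completes the animation.
; The construction script sets each stone's material color.
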(event EventEventPlaySpellAnimation
  (bind _originindex (Variables|Default|GetOriginIndex))
  (bind _transform (CallFunction|GetTileTransform _originindex))
  (Transformation|SetActorLocation (.location _transform) false false)
  (Utilities|FlowControl|Sequence
    (:then_0
      (bind (_direction _locationalpha _locationz _opacity _scale) (Timeline|Timeline_SlimeBall PlayFromStart)
        (:Update
          (Transformation|SetActorLocation (+ (Math|Vector|Lerp(Vector) (.location (CallFunction|GetTileTransform (Variables|Default|GetOriginIndex))) (.location (CallFunction|GetTileTransform (Variables|Default|GetTargetIndex))) _locationalpha) (Math|Vector|MakeVector 0.0 0.0 _locationz)) false false)
          (Rendering|Material|SetScalarParameterValueonMaterials (Variables|Default|Getstone01) "Opacity" _opacity)
          (Transformation|SetRelativeScale3D (Variables|Default|GetAnim_Scale) _scale)
          (if (>= (Components|Timeline|GetPlaybackPosition (Variables|Default|GetTimeline_SlimeBall)) 0.55)
            (Utilities|FlowControl|DoOnce false
              (:Completed
                (for _array_element (Variables|Default|GetAttackedIndexes)
                  (Default|CallOnSpellAnimationHitTile self _array_element))))))
        (:Finished
          (CallFunction|EventCompleteSpellAnimation))))
    (:then_1
      (Audio|PlaySoundatLocation "/Game/HumanVocalizations/Custom/sfx-spell-ray-ice.sfx-spell-ray-ice" (.location _transform) "0, 0, 0" 1.0 1.0 0.0 0 0 0 0))))

(fn ConstructionScript
  (|CallParentFunction)
  (Rendering|Material|SetVectorParameterValueonMaterials (Variables|Default|Getstone01) "Color" (Math|Conversions|ToVector(LinearColor) "(R=0.172549,G=0.009777,B=0.000000,A=1.000000)"))
  (Rendering|Material|SetVectorParameterValueonMaterials (Variables|Default|Getstone02) "Color" (Math|Conversions|ToVector(LinearColor) "(R=0.164706,G=0.454902,B=0.211765,A=1.000000)"))
  (Rendering|Material|SetVectorParameterValueonMaterials (Variables|Default|Getstone03) "Color" (Math|Conversions|ToVector(LinearColor) "(R=0.031373,G=0.392157,B=0.090196,A=1.000000)")))